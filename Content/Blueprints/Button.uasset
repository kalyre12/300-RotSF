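; Pushable button actor that reacts to its TheButtonWasPushed event with a click sound and a press animation.
; A box trigger enables the actor's input while the PlayerCharacter overlaps it and disables it on exit.
; BeginPlay binds the push event, whose handler plays the cue at the actor and runs a timeline driving MoveableButton's relative Y position.
; The graph itself contains no input handler or dispatcher call.
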(event `self.ReceiveBeginPlay`
  (add `self.The button was pushed!` (delegate `The button was pushed!_Event`)))

(event `The button was pushed!_Event`
  (`GameplayStatics.PlaySoundAtLocation` "/Engine/VREditor/Sounds/UI/Click_on_Button_Cue.Click_on_Button_Cue" (`self.K2_GetActorLocation`) (struct) 1.0 1.0 0.0 null null null)
  (bind (_direction _reletive_y) (`Timeline|animate button push`)
    (:`Update`
      (`SceneComponent.K2_SetRelativeLocation` (`self.moveable button`) (`KismetMathLibrary.MakeVector` 0.0 _reletive_y) false false))))

(event `self.Box.OnComponentBeginOverlap`
  (params (OverlappedComponent :type "PrimitiveComponent Object Reference") (OtherActor :type "Actor Object Reference") (OtherComp :type "PrimitiveComponent Object Reference") (OtherBodyIndex :type Integer) (bFromSweep :type Boolean) (SweepResult :type "HitResult Structure (by ref)"))
  (cast `/Game/Blueprints/PlayerAndGame/PlayerCharacter` OtherActor)
  (`self.EnableInput` (`GameplayStatics.GetPlayerController` 0)))

(event `self.Box.OnComponentEndOverlap`
  (params (OverlappedComponent :type "PrimitiveComponent Object Reference") (OtherActor :type "Actor Object Reference") (OtherComp :type "PrimitiveComponent Object Reference") (OtherBodyIndex :type Integer))
  (cast `/Game/Blueprints/PlayerAndGame/PlayerCharacter` OtherActor)
  (`self.DisableInput` (`GameplayStatics.GetPlayerController` 0)))

(fn `UserConstructionScript`)